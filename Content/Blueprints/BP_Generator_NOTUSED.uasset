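; Prototype procedural generator, marked unused by its file name, that chains piece meshes as instances; BeginPlay is empty and its InitializeMeshes call is disconnected.
; InitializeMeshes rebuilds one instanced static mesh component per piece, then a fixed debug loop repeatedly places only the first piece.
; Placement adds a randomly picked ArrowComponent socket location and doubled mesh extents to the previous position, ignoring rotation.
; A separate GravityToggle event flips gravity and physics simulation across all actors.
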(event Custom|IterateThroughPieces
  (bind _pieces (Variables|Default|GetPieces))
  (bind _meshestospawn (Variables|Default|GetMeshesToSpawn))
  (bind _output (Utilities|Array|Get(acopy) _pieces))
  (bind _value (Utilities|Map|Find _meshestospawn _output))
  ;[1 1 1] debug - replace with arguments
  (for _index (range 0 30)
    (bind (_socketlocation _socketrotation) (CallFunction|GetRandomSocketLocation _output))
    (bind (_transform _lastsocketlocation) (CallFunction|TransformMeshtoSocket _value (Variables|Default|GetLastMesh) _socketlocation _socketrotation))
    (Variables|Default|SetLastMeshSocketLocation _lastsocketlocation)
    (Components|InstancedStaticMesh|AddInstance _value _transform true)
    (Variables|Default|SetLastMesh (Variables|/Script/Engine.StaticMeshComponent|GetStaticMesh _value))))

(event Custom|InitializeMeshes
  (for _array_element (Actor|GetComponentsByClass "/Script/Engine.InstancedStaticMeshComponent")
    (Components|DestroyComponent _array_element))
  (Development|PrintString "START")
  (Utilities|Map|Clear (Variables|Default|GetMeshesToSpawn))
  (for _array_element_2 (Variables|Default|GetPieces)
    (Development|PrintString "Adding iSM")
    (bind _returnvalue (AddComponent|AddInstancedStaticMeshComponent false))
    (Components|StaticMesh|SetStaticMesh _returnvalue (Variables|/Script/Engine.StaticMeshComponent|GetStaticMesh (Variables|/Game/Blueprints/BP_Piece_NOTUSED.BP_Piece_NOTUSED_C|GetPieceMesh _array_element_2)))
    (Utilities|Map|Add (Variables|Default|GetMeshesToSpawn) _array_element_2 _returnvalue))
  (CallFunction|IterateThroughPieces))

(event Custom|GravityToggle
  (bind _isa (Utilities|FlowControl|FlipFlop)
    (:A
      _)
    (:B
      _))
  (bind _outactors (Actor|GetAllActorsOfClass "/Script/Engine.Actor"))
  (for _array_element _outactors
    (Physics|SetEnableGravity (Actor|GetComponentsByClass _array_element "/Script/Engine.PrimitiveComponent") _isa)
    (Physics|SetSimulatePhysics (Actor|GetComponentsByClass _array_element "/Script/Engine.PrimitiveComponent") _isa)))

(event Collision|EventActorBeginOverlap
  (params (OtherActor :type Actor%20Object%20Reference)))

(event EventTick
  (params (DeltaSeconds :type Float%20%28single-precision%29)))

(event EventBeginPlay)

(fn ConstructionScript)

(fn GetRandomSocketLocation
  (params (Piece :type BP%20Piece%20NOTUSED%20Object%20Reference))
  (bind _returnvalue (Actor|GetComponentsByClass Piece "/Script/Engine.ArrowComponent"))
  (for _index (range 0 (Utilities|Array|LastIndex _returnvalue))
    (if (Math|Random|RandomBool)
      (Development|PrintString (Utilities|String|Append "Using socket: " (Utilities|GetDisplayName (Utilities|Array|Get(acopy) _returnvalue _index))))
      (return (Transformation|GetWorldLocation (Utilities|Array|Get(acopy) _returnvalue _index)) (Transformation|GetWorldRotation (Utilities|Array|Get(acopy) _returnvalue _index)))))
  (Variables|Default|SetUsed2Sockets true))

(fn TransformMeshtoSocket
  (params (MeshReference :type Instanced%20Static%20Mesh%20Component%20Object%20Reference) (LastMesh :type Static%20Mesh%20Object%20Reference) (SocketLocation :type Vector) (SocketRotation :type Rotator))
  (bind _staticmesh (Variables|/Script/Engine.StaticMeshComponent|GetStaticMesh MeshReference))
  (bind _lastmeshsocketlocation (Variables|Default|GetLastMeshSocketLocation))
  (bind _returnvalue (StaticMesh|GetBounds _staticmesh))
  (bind _returnvalue_2 (+ SocketLocation _lastmeshsocketlocation))
  (bind _returnvalue_3 (* (.boxextent _returnvalue) "2.000000,2.000000,2.000000"))
  (bind _returnvalue_4 (+ _returnvalue_3 _returnvalue_2))
  (return (Math|Transform|MakeTransform _returnvalue_4) _returnvalue_4))